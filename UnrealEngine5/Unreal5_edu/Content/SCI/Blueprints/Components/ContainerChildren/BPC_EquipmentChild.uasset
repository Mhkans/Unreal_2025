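; Equipment container component, a child of a base container, that restricts each slot to items of the matching equipment type.
; When the parent's drop handling returns false, it validates the item's type tag and the slot's entry in EquipmentSlotOrder before transferring it.
; EquipmentSlotOrder must match UI slot indices.
; Add and remove overrides fire equipment added and removed notifications; the drop path's own added call is disconnected.
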(fn DropItemonSlot
  (params (FromContainer :type BPC%20Container%20Object%20Reference) (TargetIndex :type Integer) (FromIndex :type Integer))
  ;[1 1 1] Confirms that the incoming item is both equipment and equipment of the correct type for the slot prior to attempting to move it
  (bind _sameslot (|CallParentFunction FromContainer TargetIndex FromIndex))
  (if (not _sameslot)
    (bind _success (CallFunction|ValidSlotTypeforItem (Default|GetItematIndex FromContainer FromIndex) TargetIndex))
    (if _success
      (bind _itemsswapped (Default|TransferItem FromContainer self TargetIndex FromIndex)))))

(fn ValidateEquipmentSlot
  (params (Index :type Integer) (IncomingItem :type STR%20Item%20Data%20Structure))
  ;[1 1 1] Confirms that the incoming items equipable type matches the equipment slot type at the same index. Equipment Slot Order must match UI Slot Index.
  (return (== "" (Utilities|Array|Get(acopy) (Variables|Default|GetEquipmentSlotOrder) Index))))

(fn ValidSlotTypeforItem
  (params (Item :type STR%20Item%20Data%20Structure) (Index :type Integer))
  ;[1 1 1] Confirms item matches equipment requirements
  (return (and (GameplayTags|HasTag (Variables|Default|GetValidItemTypes) (Utilities|Struct|BreakSTR_ItemData Item) true) (== "" (Utilities|Array|Get(acopy) (Variables|Default|GetEquipmentSlotOrder) Index)))))

(fn AddItemtoIndex
  (params (Index :type Integer) (Item :type STR%20Item%20Data%20Structure%20%28by%20ref%29))
  (|CallParentFunction Index Item)
  (Default|CallOnEquipmentAdded Index)
  (return))

(fn RemoveItematIndex
  (params (Index :type Integer))
  (Default|CallOnEquipmentRemoved (CallFunction|GetItematIndex Index))
  (|CallParentFunction Index))