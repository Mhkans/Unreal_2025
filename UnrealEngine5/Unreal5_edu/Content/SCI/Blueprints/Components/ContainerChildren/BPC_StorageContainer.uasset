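; BPC_StorageContainer is a child container component for item storage that can restrict which item types it accepts.
; Dropping an item runs the parent logic first and, if that returns false, has the source container transfer the item to the target slot.
; Slot validation requires an exact match in the ValidItemTypes gameplay tags, or accepts any item when that list is empty.
; The player save and load interface functions are empty overrides.
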(event EventTick
  (params (DeltaSeconds :type Float%20%28single-precision%29)))

(fn DropItemonSlot
  (params (FromContainer :type BPC%20Container%20Object%20Reference) (TargetIndex :type Integer) (FromIndex :type Integer))
  ;[1 1 1] After running parent function, transfers the item
  (bind _sameslot (|CallParentFunction FromContainer TargetIndex FromIndex))
  (if (not _sameslot)
    (Default|TransferItem FromContainer self TargetIndex FromIndex)
    (return false)))

(fn SavePlayerDataBPI
  (return))

(fn GetPlayerSaveBPI
  (return))

(fn LoadPlayerDataBPI
  (return))

(fn ValidSlotTypeforItem
  (params (Item :type STR%20Item%20Data%20Structure) (Index :type Integer))
  ;[1 1 1] Checks if the container has any valid item types and if so, checks them.
  (if (> (GameplayTags|GetNumGameplayTagsinContainer (Variables|Default|GetValidItemTypes)) 0)
    (return (GameplayTags|HasTag (Variables|Default|GetValidItemTypes) (Utilities|Struct|BreakSTR_ItemData Item) true))
    (else
      (return true))))