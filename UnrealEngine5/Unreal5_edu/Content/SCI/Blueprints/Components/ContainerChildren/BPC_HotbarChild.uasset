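; Hotbar variant of the item container component, restricting which item types can be dropped into hotbar slots.
; When the parent drop logic returns false, it transfers the item only if its type tag exactly matches the ValidItemTypes container.
; A lookup returns the item and type tag at a valid hotbar index.
; Removal just calls the parent, as the hotbar update and slot-check interface messages are not wired in.
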(fn DropItemonSlot
  (params (FromContainer :type BPC%20Container%20Object%20Reference) (TargetIndex :type Integer) (FromIndex :type Integer))
  ;[1 1 1] After running parent function, checks if the item can be added to the hotbar and transfers it if it can.
  (bind _sameslot (|CallParentFunction FromContainer TargetIndex FromIndex))
  (if (not _sameslot)
    (LocalVariables|SetLocalItem (Default|GetItematIndex FromContainer FromIndex))
    (bind _success (CallFunction|ValidSlotTypeforItem (LocalVariables|GetLocalItem)))
    (if _success
      (Default|TransferItem FromContainer self TargetIndex FromIndex))))

(fn GetHotbarIndex
  (params (Index :type Integer))
  (bind _items (Variables|Default|GetItems))
  (bind _output (Utilities|Array|Get(acopy) _items Index))
  ;[1 1 1] Checks for valid item in the hotbar and returns it's item type tag
  (if (Utilities|Array|IsValidIndex _items Index)
    (if (CallFunction|ItemIsValid _output)
      (return true (Utilities|Struct|BreakSTR_ItemData _output) _output)
      (else
        (return false "" "")))))

(fn ValidSlotTypeforItem
  (params (Item :type STR%20Item%20Data%20Structure) (Index :type Integer))
  ;[1 1 1] Confirms item matches hotbar requirements
  (return (GameplayTags|HasTag (Variables|Default|GetValidItemTypes) (Utilities|Struct|BreakSTR_ItemData Item) true)))

(fn RemoveItematIndex
  (params (Index :type Integer))
  ;[1 1 1] Checks hotbar for equipped items when removing from it
  (|CallParentFunction Index))