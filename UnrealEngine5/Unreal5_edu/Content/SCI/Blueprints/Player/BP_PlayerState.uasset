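; Player State Blueprint that initializes each player's Inventory and Hotbar components once that player is ready.
; A looping timer started on BeginPlay polls IsStateReady, then clears itself and calls a server event to initialize both components.
; Remote clients query their HUD through an interface message and report load status by server RPC.
; The server waits on that flag for connecting clients, while the host is ready immediately.
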(event Custom|SetHUDLoaded%20%28Server%29
  (params (Loaded :type Boolean))
  ;[1 1 1] Sets up the Player State for each player
  (Variables|Default|SetHUDLoaded Loaded))

(event Custom|InitPlayerComponents%20%28Server%29
  ;[1 1 1] Sets up the Player State for each player
  (CallFunction|InitPlayerComponents))

(event Custom|InitializationHandle
  ;[1 1 1] Sets up the Player State for each player
  (bind _returnvalue (CallFunction|IsStateReady))
  (if _returnvalue
    (Utilities|Time|ClearandInvalidateTimerbyHandle (Variables|Default|GetInitializationTimer))
    (CallFunction|InitPlayerComponents(Server))))

(event EventBeginPlay
  (bind _returnvalue (Game|GetPlayerController))
  ;[1 1 1] Sets up the Player State for each player
  (Utilities|IsValid _returnvalue
    (:Is%20Valid
      (Variables|Default|SetHUD (HUD|GetHUD _returnvalue))
      (bind _returnvalue_2 (Utilities|Time|SetTimerbyEvent (delegate Custom|InitializationHandle) 0.2 true))
      (Variables|Default|SetInitializationTimer _returnvalue_2))))

(fn ConstructionScript)

(fn IsStateReady
  ;[1 1 1] Confirms Client is correctly initialized
  (Networking|SwitchHasAuthority
    (:Authority
      (if (and (Networking|IsServer) (not (Pawn|IsLocalController (Game|GetPlayerController))))
        (if (Variables|Default|GetHUDLoaded) ; If Client, wait until loaded to init server side
          (return true)
          (else
            (return false)))
        (else
          (return true) ; If Host, always return true
        )))
    (:Remote
      (bind _complete (Class|BPIHUD|ClientInitCompleteBPI(Message) (Variables|Default|GetHUD)))
      (CallFunction|SetHUDLoaded(Server) _complete)
      (return _complete))))

(fn InitPlayerComponents
  ;[1 1 1] Sets up the inventory & hotbar
  (Default|InitComponent (Variables|Default|GetInventory) 10)
  (Default|InitComponent (Variables|Default|GetHotbar) 8))

(fn UpdateUIComponents
  (params (InventorySlots :type Integer)))