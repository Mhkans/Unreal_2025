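; Interactable loot container (chest) that players toggle open and closed, with a world marker showing the open/close prompt.
; Interaction adds or removes the player through server RPCs, updates the open state and toggles that player's container UI.
; On first interaction it rolls a data-table loot list by drop chance and quantity into its storage component.
; Storage changes refresh the inventory UI of every player using it.
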(event Custom|UpdateContainerUI
  (params (Item :type STR%20Item%20Data%20Structure) (Add :type Boolean))
  ;[1 1 1] Updates the UI when the container changes
  (for _array_element (Variables|Default|GetUsingPlayers)
    (bind _asbp_player_controller (Utilities|Casting|CastToBP_PlayerController _array_element))
    (Default|UpdateContainerUI(Server) (Variables|/Game/SCI/Blueprints/Player/BP_PlayerController.BP_PlayerController_C|GetInventoryMaster _asbp_player_controller) "(TagName=\"Items.Container.Storage\")")))

(event Custom|RemoveUsingPlayer%20%28Server%29
  (params (Player :type Player%20Controller%20Object%20Reference%20%28by%20ref%29))
  (bind _usingplayers (Variables|Default|GetUsingPlayers))
  ;[1 1 1] Adds/Removes player from the container
  (Utilities|Array|RemoveItem _usingplayers Player)
  (CallFunction|UpdateOpen(Client) (not (Utilities|Array|IsEmpty _usingplayers))))

(event Custom|AddUsingPlayer%20%28Server%29
  (params (Player :type Player%20Controller%20Object%20Reference%20%28by%20ref%29))
  ;[1 1 1] Adds/Removes player from the container
  (Utilities|Array|Add (Variables|Default|GetUsingPlayers) Player)
  (CallFunction|UpdateOpen(Client) true))

(event Custom|SpawnItemsInContainer
  ;[1 1 1] Spawns items on first open
  (if (Variables|Default|GetSpawnItems)
    (CallFunction|SpawnItemsfromList)))

(event Custom|UpdateOpen%20%28Client%29
  (params (IsOpen :type Boolean))
  ;[1 1 1] Sets is open or not
  (Variables|Default|SetIsOpen IsOpen)
  (Default|UpdateName (Variables|Default|GetMarkerWidget) (select (Variables|Default|GetIsOpen) "Close Chest" "Open Chest") false))

(event EventLookingatBPI
  (params (LookingAt :type Boolean))
  ;[1 1 1] World Widget
  (Development|SetHiddeninGame (Variables|Default|GetMarker) (not LookingAt) false))

(event EventSetInteractionTextBPI
  ;[1 1 1] World Widget
  (Default|UpdateName (Variables|Default|GetMarkerWidget) (select (Variables|Default|GetIsOpen) "Close Chest" "Open Chest") false))

(event EventTriggerInteractionBPI
  (params (PlayerController :type Player%20Controller%20Object%20Reference) (PlayerCharacter :type BP%20Player%20Character%20Object%20Reference))
  ;[1 1 1] Adds a removes a player when interacting and toggles the UI
  (if (Utilities|Array|ContainsItem (Variables|Default|GetUsingPlayers) PlayerController)
    (CallFunction|RemoveUsingPlayer(Server) PlayerController)
    (else
      (CallFunction|AddUsingPlayer(Server) PlayerController)))
  (Class|BPIPlayerController|ToggleContainerUIBPI(Message) PlayerController self (Variables|Default|GetTotal%20Slots) (Variables|Default|GetContainer%20Name) true)
  (CallFunction|SpawnItemsinContainer))

(event EventBeginPlay
  ;[1 1 1] Sets up the container component and the marker widget
  (Default|InitComponent (Variables|Default|GetStorageContainer) (Variables|Default|GetTotal%20Slots))
  (EventDispatchers|BindEventtoOnItemChanged (Variables|Default|GetStorageContainer) (EventDispatchers|CreateEvent :!event Custom|UpdateContainerUI))
  (bind _asui_marker (Utilities|Casting|CastToUI_Marker (UserInterface|GetWidget (Variables|Default|GetMarker))))
  (Variables|Default|SetMarkerWidget _asui_marker))

(fn ConstructionScript)

(fn SpawnItemsfromList
  (bind _spawnlist (Variables|Default|GetSpawnList))
  ;[1 1 1] Checks the loot table intended to drop and rolls against the drop chance, adding the items to the container if successful.
  (bind _returnvalue (Utilities|GetDataTableRow (.datatable _spawnlist) (.rowname _spawnlist))
    (:then
      (for _array_element (.LootItems (Utilities|Struct|BreakSTR_DropTables _returnvalue))
        (if (>= (.DropChance (Utilities|Struct|BreakSTR_LootItems _array_element)) (Math|Random|RandomFloatinRange 0.0 1.0))
          (bind _returnvalue_2 (Utilities|GetDataTableRow (.DataTable (Utilities|Struct|BreakDataTableRowHandle (.Item (Utilities|Struct|BreakSTR_LootItems _array_element)))) (.RowName (Utilities|Struct|BreakDataTableRowHandle (.Item (Utilities|Struct|BreakSTR_LootItems _array_element)))))
            (:then
              (LocalVariables|SetLocalItem _returnvalue_2)
              (bind _structout (Utilities|Struct|SetmembersinSTR_ItemData (LocalVariables|GetLocalItem) (Utilities|Struct|MakeSTR_ItemValues (Math|Random|RandomIntegerinRange (.MinDrop (Utilities|Struct|BreakSTR_LootItems _array_element)) (.MaxDrop (Utilities|Struct|BreakSTR_LootItems _array_element))))))
              (Default|AddItemtoContainer (Variables|Default|GetStorageContainer) _structout)))))
      (Variables|Default|SetSpawnItems false))))

(fn CheckInteractableBPI
  (return true 0.0))

(fn ShouldOutlineBPI
  (return true))