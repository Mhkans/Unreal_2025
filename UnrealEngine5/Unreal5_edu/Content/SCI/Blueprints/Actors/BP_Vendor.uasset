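; BP_Vendor is an interactable vendor actor that opens and closes its shop through a VendorComponent when a player triggers interaction.
; It implements interaction interface calls, always allowing instant interaction and never requesting an outline.
; On BeginPlay it caches the UI_Marker from its world-space widget, which shows a "Vendor" label and is visible only while the player looks at it.
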(event EventLookingatBPI
  (params (LookingAt :type Boolean))
  ;[1 1 1] World Widget
  (Development|SetHiddeninGame (Variables|Default|GetMarker) (not LookingAt) false))

(event EventBeginPlay
  ;[1 1 1] World Widget
  (bind _asui_marker (Utilities|Casting|CastToUI_Marker (UserInterface|GetWidget (Variables|Default|GetMarker))))
  (Variables|Default|SetMarkerWidget _asui_marker))

(event EventSetInteractionTextBPI
  ;[1 1 1] World Widget
  (Default|UpdateName (Variables|Default|GetMarkerWidget) "Vendor" false))

(event EventTriggerInteractionBPI
  (params (PlayerController :type Player%20Controller%20Object%20Reference) (PlayerCharacter :type BP%20Player%20Character%20Object%20Reference))
  (Default|ToggleVendor (Variables|Default|GetVendorComponent) PlayerController))

(fn ConstructionScript)

(fn CheckInteractableBPI
  (return true 0.0))

(fn ShouldOutlineBPI
  (return false))